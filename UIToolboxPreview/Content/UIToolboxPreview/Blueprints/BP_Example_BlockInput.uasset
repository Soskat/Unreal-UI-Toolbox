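; UI Toolbox preview example Blueprint that blocks game input while a widget is open.
; On execute, it pushes the example widget class to a tagged UI layer for the local player, focuses it and shows the cursor.
; Widget deactivation restores game-only input, hides the cursor and clears the reference.
; Despite its name, SwitchToGameAndUIInputMode sets UI-only input.
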(event Custom|OnCachedWidgetDeactivated
  (Utilities|IsValid (Variables|Default|GetUI_Example)
    (:Is%20Valid
      (CallFunction|SwitchtoGameOnlyInputMode)
      (Variables|Default|SetUI_Example 0))))

(event EventOnExecuteExample
  (bind _ui_example (Variables|Default|GetUI_Example))
  (CallFunction|SpawnWidgetExample)
  (Utilities|IsValid _ui_example
    (:Is%20Valid
      (EventDispatchers|BindEventtoBPonWidgetDeactivated _ui_example (delegate Custom|OnCachedWidgetDeactivated))
      (CallFunction|SwitchtoGameandUIInputMode (Variables|Default|GetUI_Example)))))

(fn ConstructionScript)

(fn SpawnWidgetExample
  (bind _returnvalue (Game|GetPlayerController 0))
  (Utilities|IsValid _returnvalue
    (:Is%20Valid
      (bind _returnvalue_2 (Class|CoreUIUtils|GetLocalPlayerfromController _returnvalue))
      (Utilities|IsValid _returnvalue_2
        (:Is%20Valid
          (bind _returnvalue_3 (Class|CoreUIUtils|PushContenttoLayerforPlayer _returnvalue_2 (Variables|Default|GetLayerNameTag) (Variables|Default|GetWidgetExampleClass)))
          (Variables|Default|SetUI_Example _returnvalue_3)
          (return))))))

(fn SwitchtoGameOnlyInputMode
  (bind _returnvalue (Game|GetPlayerController 0))
  (Utilities|IsValid _returnvalue
    (:Is%20Valid
      (Input|SetInputModeGameOnly _returnvalue false)
      (Variables|/Script/Engine.PlayerController|SetbShowMouseCursor _returnvalue false))))

(fn SwitchtoGameandUIInputMode
  (params (InWidgetToFocus :type Widget%20Object%20Reference))
  (bind _returnvalue (Game|GetPlayerController 0))
  (Utilities|IsValid _returnvalue
    (:Is%20Valid
      (Input|SetInputModeUIOnly _returnvalue InWidgetToFocus "DoNotLock" false)
      (Variables|/Script/Engine.PlayerController|SetbShowMouseCursor _returnvalue true))))